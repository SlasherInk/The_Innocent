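; Bathroom stall door Blueprint that swings open or closed each time its OpenDoor event is called.
; A FlipFlop alternates between playing and reversing a timeline, which lerps the StallDoor's relative yaw to swing it.
; Opening plays the open sound at once, while closing waits a short delay before playing the close sound, each stopping the other.
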(event Custom|OpenDoor
  (Utilities|FlowControl|FlipFlop
    (:A
      (Audio|Components|Audio|Stop (Variables|Default|GetStallDoorClose))
      (Audio|Components|Audio|Play (Variables|Default|GetStallDoorOpen) 0.0)
      (bind _dooropen (Timeline|Open%20Door Play)
        (:Update
          (Transformation|SetRelativeRotation (Variables|Default|GetStallDoor) (Math|Rotator|MakeRotator 0.0 0.0 (Math|Float|Lerp 0.0 -8e+01 _dooropen)) false false))))
    (:B
      (Utilities|FlowControl|Sequence
        (:then_0
          (Timeline|Open%20Door Reverse))
        (:then_1
          (Utilities|FlowControl|Delay 0.7)
          (Audio|Components|Audio|Stop (Variables|Default|GetStallDoorOpen))
          (Audio|Components|Audio|Play (Variables|Default|GetStallDoorClose) 0.0))))))

(fn ConstructionScript)