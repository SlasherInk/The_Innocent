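; Desk puzzle actor that the player rotates in 90-degree yaw steps until the step count matches PuzzleAnswer.
; Overlapping binds Desk_Rotate to the player's interact event unless already finalized, and leaving unbinds it.
; A timeline animates each turn while DeskMoving blocks overlapping turns, then increments DeskPosition, which never wraps.
; On a match it sets Finalized, plays a sound and calls EVDPuzzleCompleted.
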(event Custom|Desk_Rotate
  (params (isPressed :type Boolean))
  (if (not (Variables|Default|GetDeskMoving))
    (Variables|Default|SetDeskMoving true)
    (Audio|PlaySound2D 0 1.0 1.0 0.0 0 0)
    (bind _rotation (Timeline|DeskRotation PlayFromStart)
      (:Update
        (Transformation|SetRelativeRotation (Variables|Default|GetDesk) (Math|Rotator|MakeRotator 0.0 0.0 (Math|Float|Lerp (.yaw (Variables|Default|GetStartingRotationDesk)) (+ (.yaw (Variables|Default|GetStartingRotationDesk)) 9e+01) _rotation)) false false))
      (:Finished
        (Variables|Default|SetStartingRotationDesk (Math|Rotator|MakeRotator 0.0 0.0 (Math|Float|Lerp (.yaw (Variables|Default|GetStartingRotationDesk)) (+ (.yaw (Variables|Default|GetStartingRotationDesk)) 9e+01) _rotation)))
        (Variables|Default|SetDeskMoving false)
        (bind _result (Math|Integer|IncrementInt (Variables|Default|GetDeskPosition))
          (:%20%20
            (Variables|Default|SetDeskPosition _result)
            ;[0 0 0 0.5] Check Puzzle by Rotation Position
            (if (== (Variables|Default|GetPuzzleAnswer) (Variables|Default|GetDeskPosition))
              (Development|PrintString "Puzzle Finished")
              (Variables|Default|SetFinalized true)
              (Audio|PlaySound2D 0 1.0 1.0 0.0 0 0)
              (Default|CallEVDPuzzleCompleted))))))))

(event EventBeginPlay
  (Variables|Default|SetStartingRotationDesk (Variables|/Script/Engine.SceneComponent|GetRelativeRotation (Variables|Default|GetDesk)))
  (bind _asbp_gm_gameplay (Utilities|Casting|CastToBP_GM_Gameplay (Game|GetGameMode)))
  (Variables|Default|SetMyGameMode _asbp_gm_gameplay))

(event Collision|EventActorBeginOverlap
  (params (OtherActor :type Actor%20Object%20Reference))
  (bind _ascharacter_player (Utilities|Casting|CastToCharacter_Player OtherActor))
  (if (not (Variables|Default|GetFinalized))
    (EventDispatchers|BindEventtoInteract _ascharacter_player (delegate Custom|Desk_Rotate))))

(event Collision|EventActorEndOverlap
  (params (OtherActor :type Actor%20Object%20Reference))
  (bind _ascharacter_player (Utilities|Casting|CastToCharacter_Player OtherActor))
  (EventDispatchers|UnbindallEventsfromInteract _ascharacter_player))

(event Input|KeyboardEvents|E
  (params (Key :type Key%20Structure :default "None"))
  ;[0 0 0 0.5] Call Interact
  (:Pressed
    (Default|CallInteract true))
  (:Released
    (Default|CallInteract false)))

(fn ConstructionScript
  (|CallParentFunction))