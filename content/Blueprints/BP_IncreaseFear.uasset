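; BP_IncreaseFear is a pickup that gives Character_Player the IncreaseFear item or ability on a right mouse click.
; A sphere overlap enables the actor's input while the player is inside and disables it on exit.
; The click sets the player's HasIncreaseFear flag, destroys the pickup's IncreaseFear component and reveals the matching component on the player, leaving the pickup actor itself in place.
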(event OnComponentBeginOverlap(Sphere)
  (params (OverlappedComponent :type Primitive%20Component%20Object%20Reference) (OtherActor :type Actor%20Object%20Reference) (OtherComp :type Primitive%20Component%20Object%20Reference) (OtherBodyIndex :type Integer) (bFromSweep :type Boolean) (SweepResult :type Hit%20Result%20Structure%20%28by%20ref%29))
  (Utilities|Casting|CastToCharacter_Player OtherActor)
  (Input|EnableInput (Game|GetPlayerController 0)))

(event OnComponentEndOverlap(Sphere)
  (params (OverlappedComponent :type Primitive%20Component%20Object%20Reference) (OtherActor :type Actor%20Object%20Reference) (OtherComp :type Primitive%20Component%20Object%20Reference) (OtherBodyIndex :type Integer))
  (Utilities|Casting|CastToCharacter_Player OtherActor)
  (Input|DisableInput (Game|GetPlayerController 0)))

(event EventBeginPlay)

(event Collision|EventActorBeginOverlap
  (params (OtherActor :type Actor%20Object%20Reference)))

(event EventTick
  (params (DeltaSeconds :type Float%20%28single-precision%29)))

(event Input|KeyboardEvents|E
  (params (Key :type Key%20Structure :default "None")))

(event Input|MouseEvents|RightMouseButton
  (params (Key :type Key%20Structure :default "None"))
  (:Pressed
    (bind _ascharacter_player (Utilities|Casting|CastToCharacter_Player (stale OnComponentBeginOverlap(Sphere) OtherActor)))
    (Variables|/Game/CharacterCustomization/Blueprints/Character_Player.Character_Player_C|SetHas%20increaseFear? _ascharacter_player true)
    (Components|DestroyComponent (Variables|Default|GetincreaseFear))
    (Rendering|SetVisibility (Variables|/Game/CharacterCustomization/Blueprints/Character_Player.Character_Player_C|GetincreaseFear _ascharacter_player) true false)))

(fn ConstructionScript)