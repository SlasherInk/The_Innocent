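; BP_GameSettings spawns Innocent and Shadow characters at level start, then gives player 0 control of one matching CharacterType.
; SpawnPlayers places InnocentCount innocents at the first PlayerStartsL entries and ShadowCount shadows at those following, skipping invalid indices.
; It gathers and shuffles the PlayerStart actors only after those spawn loops, so spawning reads the array's prior contents.
; BeginPlay then possesses a random actor of the chosen class.
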(event EventBeginPlay
  (Utilities|FlowControl|Sequence
    (:then_0
      (CallFunction|SpawnPlayers))
    (:then_1
      (switch Utilities|FlowControl|Switch|Switchone_CharacterType (Variables|Default|GetCharacterType)
        (:NewEnumerator1
          (bind _outactors (Actor|GetAllActorsOfClass "/Game/CharacterCustomization/Blueprints/BP_Innocent.BP_Innocent_C"))
          (Pawn|Possess (Game|GetPlayerController 0) (Utilities|Array|Get(acopy) _outactors (Math|Random|RandomInteger (Utilities|Array|Length _outactors)))))
        (:NewEnumerator2
          (bind _outactors_2 (Actor|GetAllActorsOfClass "/Game/CharacterCustomization/Blueprints/BP_Shadow.BP_Shadow_C"))
          (Pawn|Possess (Game|GetPlayerController 0) (Utilities|Array|Get(acopy) _outactors_2 (Math|Random|RandomInteger (Utilities|Array|Length _outactors_2)))))))))

(fn ConstructionScript)

(fn SpawnPlayers
  (Utilities|FlowControl|Sequence
    (:then_0
      (Utilities|FlowControl|Sequence
        (:then_0
          (for _index (range 0 (- (Variables|Default|GetInnocentCount) 1))
            (if (Utilities|Array|IsValidIndex (LocalVariables|GetplayerStarts_l) _index)
              (Game|SpawnActorfromClass "/Game/CharacterCustomization/Blueprints/BP_Innocent.BP_Innocent_C" (Math|Transform|MakeTransform (Transformation|GetActorLocation (Utilities|Array|Get(acopy) (LocalVariables|GetplayerStarts_l) _index)) (Transformation|GetActorRotation (Utilities|Array|Get(acopy) (LocalVariables|GetplayerStarts_l) _index))) "Undefined" "MultiplyWithRoot" 0 0))))
        (:then_1
          (for _index_2 (range 0 (- (Variables|Default|GetShadowCount) 1))
            (if (Utilities|Array|IsValidIndex (LocalVariables|GetplayerStarts_l) (+ (Variables|Default|GetInnocentCount) _index_2))
              (Game|SpawnActorfromClass "/Game/CharacterCustomization/Blueprints/BP_Shadow.BP_Shadow_C" (Math|Transform|MakeTransform (Transformation|GetActorLocation (Utilities|Array|Get(acopy) (LocalVariables|GetplayerStarts_l) (+ (Variables|Default|GetInnocentCount) _index_2))) (Transformation|GetActorRotation (Utilities|Array|Get(acopy) (LocalVariables|GetplayerStarts_l) (+ (Variables|Default|GetInnocentCount) _index_2)))) "Undefined" "MultiplyWithRoot" 0 0))))))
    (:then_1
      (bind _outactors (Actor|GetAllActorsOfClass "/Script/Engine.PlayerStart"))
      (LocalVariables|SetplayerStarts_l _outactors)
      (Utilities|Array|Shuffle (LocalVariables|GetplayerStarts_l)))))