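; Character customization component that frames the owner's named camera on a bone of its named skeletal mesh and can make the owner the view target.
; SetCameraTarget snaps or curve-blends camera position and mesh yaw to the given settings; afterwards, interpolation keeps the camera tracking the bone.
; Touch drags smoothly spin the mesh through a runtime-added parent scene component, with a timer started on release to reset the rotation.
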(fn FindSkeletalMesh
  (for _array_element (Actor|GetComponentsByClass (Components|GetOwner) "/Script/Engine.SkeletalMeshComponent")
    (if (Utilities|Enum|Equal(Enum) (Utilities|GetObjectName _array_element) (Variables|CustomizationCamera|GetMeshComponentName))
      (Variables|CustomizationCamera|Main|SetRootSkeletalMeshComponent _array_element)
      (return true))))

(fn FindCamera
  (for _array_element (Actor|GetComponentsByClass (Components|GetOwner) "/Script/Engine.CameraComponent")
    (if (Utilities|Enum|Equal(Enum) (Utilities|GetObjectName _array_element) (Variables|CustomizationCamera|GetCameraComponentName))
      (Variables|CustomizationCamera|Main|SetCamera _array_element)
      (return true))))

(fn SetCameraTarget
  (params (Settings :type Struct%20Camera%20Settings%20Structure) (Instant :type Boolean))
  (bind _camera (Variables|CustomizationCamera|Main|GetCamera))
  (bind _returnvalue (Transformation|GetRelativeTransform _camera))
  (Variables|CustomizationCamera|Data|SetCurrentSettings Settings)
  (Utilities|FlowControl|Sequence
    (:then_0
      (Variables|CustomizationCamera|Data|SetCameraStartLocation (.location _returnvalue))
      (Variables|CustomizationCamera|Data|SetCameraStartRotation (.rotation _returnvalue))
      (Variables|CustomizationCamera|Data|SetCharacterStartRotation (Variables|/Script/Engine.SceneComponent|GetRelativeRotation (Variables|CustomizationCamera|Main|GetRootSkeletalMeshComponent)))
      (Variables|CustomizationCamera|Data|SetCameraCurveTime 0.0))
    (:then_1
      (if Instant
        (CustomizationCamera|Update|UpdateCameraPosition 1.0)
        (else
          (Variables|CustomizationCamera|Data|SetUpdateCameraPosition true))))))

(fn UpdateCameraPosition
  (params (Alpha :type Float%20%28single-precision%29))
  (bind _returnvalue (Components|GetOwner))
  (bind _rootskeletalmeshcomponent (Variables|CustomizationCamera|Main|GetRootSkeletalMeshComponent))
  (bind _rootskeletalmeshcomponent_2 (Variables|CustomizationCamera|Main|GetRootSkeletalMeshComponent))
  (bind _currentsettings (Variables|CustomizationCamera|Data|GetCurrentSettings))
  (bind _currentsettings_2 (Variables|CustomizationCamera|Data|GetCurrentSettings))
  (bind _bonetotrack (Utilities|Struct|BreakStruct_CameraSettings _currentsettings))
  (bind _offset (Utilities|Struct|BreakStruct_CameraSettings _currentsettings_2))
  (bind _origin (Collision|GetComponentBounds _rootskeletalmeshcomponent))
  (bind _returnvalue_2 (Transformation|GetActorRightVector _returnvalue))
  (bind _returnvalue_3 (Transformation|GetActorForwardVector _returnvalue))
  (bind (_x _y _z) (Math|Vector|BreakVector _offset))
  (bind _returnvalue_4 (Math|Vector|NegateVector _returnvalue_3))
  (bind _returnvalue_5 (Transformation|GetSocketTransform _rootskeletalmeshcomponent_2 _bonetotrack "RTS_Actor"))
  (bind _returnvalue_6 (* _returnvalue_4 _x))
  (bind _returnvalue_7 (* _returnvalue_2 _y))
  (bind _returnvalue_8 (+ (.location _returnvalue_5) _returnvalue_6 _returnvalue_7))
  (bind (_x_2 _y_2) (Math|Vector|BreakVector _returnvalue_8))
  (Transformation|SetRelativeLocation (Variables|CustomizationCamera|Main|GetCamera) (Math|Vector|Lerp(Vector) (Variables|CustomizationCamera|Data|GetCameraStartLocation) (Math|Vector|MakeVector _x_2 _y_2 (+ (+ (.Z (Math|Vector|BreakVector _origin)) (Math|Float|Absolute(Float) (.Z (Math|Vector|BreakVector (- _origin (Transformation|GetSocketLocation (Variables|CustomizationCamera|Main|GetRootSkeletalMeshComponent) (Utilities|Struct|BreakStruct_CameraSettings (Variables|CustomizationCamera|Data|GetCurrentSettings)))))))) _z)) Alpha) false false)
  (Transformation|SetRelativeRotation (Variables|CustomizationCamera|Main|GetRootSkeletalMeshComponent) (Math|Rotator|MakeRotator 0.0 0.0 (.yaw (Math|Rotator|Lerp(Rotator) (Variables|CustomizationCamera|Data|GetCharacterStartRotation) (Math|Rotator|MakeRotator 0.0 0.0 (+ (+ (.Yaw (Math|Rotator|BreakRotator (Math|Rotator|FindLookatRotation (Transformation|GetWorldLocation (Variables|CustomizationCamera|Main|GetRootSkeletalMeshComponent)) (Transformation|GetWorldLocation (Variables|CustomizationCamera|Main|GetCamera))))) 9e+01) (Utilities|Struct|BreakStruct_CameraSettings (Variables|CustomizationCamera|Data|GetCurrentSettings)))) Alpha true))) false false))

(fn UpdateCameraCurve
  (bind _cameracurve (Variables|CustomizationCamera|GetCameraCurve))
  (bind (_minvalue _maxvalue) (Class|CurveBase|GetValueRange _cameracurve))
  (Utilities|FlowControl|Sequence
    (:then_0
      (LocalVariables|SetLocAlpha (Math|Float|NormalizetoRange (Math|Curves|GetFloatValue (Variables|CustomizationCamera|GetCameraCurve) (Variables|CustomizationCamera|Data|GetCameraCurveTime)) _minvalue _maxvalue))
      (CustomizationCamera|Update|UpdateCameraPosition (LocalVariables|GetLocAlpha))
      (Math|Float|CompareFloat (LocalVariables|GetLocAlpha) 1.0
        (:==
          (return true))))
    (:then_1
      (Variables|CustomizationCamera|Data|SetCameraCurveTime (Math|Float|Min(Float) (+ (Variables|CustomizationCamera|Data|GetCameraCurveTime) (Utilities|Time|GetWorldDeltaSeconds)) (.MaxTime (Math|Curves|GetTimeRange (Variables|CustomizationCamera|GetCameraCurve))))))))

(fn ReceiveBeginPlay
  (Utilities|FlowControl|Sequence
    (:then_0
      (bind _returnvalue (CustomizationCamera|Main|FindSkeletalMesh))
      (if _returnvalue
        (bind _returnvalue_2 (Game|AddComponentbyClass (Components|GetOwner) "/Script/Engine.SceneComponent" false))
        (Variables|CustomizationCamera|Main|SetMeshRoot _returnvalue_2)
        (Transformation|AttachComponentToComponent (Variables|CustomizationCamera|Main|GetRootSkeletalMeshComponent) (Variables|CustomizationCamera|Main|GetMeshRoot) "None" "SnapToTarget" "KeepRelative" "KeepWorld" true)))
    (:then_1
      (bind _returnvalue_3 (CustomizationCamera|Main|FindCamera))
      (if _returnvalue_3
        (Transformation|SetWorldRotation (Variables|CustomizationCamera|Main|GetCamera) (Math|Conversions|RotationFromXVector (Math|Vector|NegateVector (Transformation|GetActorForwardVector (Components|GetOwner)))) false false)
        (CustomizationCamera|SetCameraTarget (Variables|CustomizationCamera|GetDefaultCameraSettings) true)
        (Class|KismetSystemLibrary|SetTimerforNextTick 0 "Try_SetViewTarget")))))

(fn UpdateTouchDelta
  (params (Delta :type Vector%202D%20Structure))
  (Variables|CustomizationCamera|TouchDrag|SetLast_TouchDelta (Class|KismetMathLibrary|ClampAxes2D Delta -1e+01 1e+01)))

(fn SetDragging
  (params (IsDragging :type Boolean))
  (bind _output_get (Variables|CustomizationCamera|TouchDrag|SetIsDragging IsDragging))
  (if _output_get
    (Utilities|Time|ClearandInvalidateTimerbyHandle (Variables|CustomizationCamera|TouchDrag|GetRootOffsetReset_TimerHandle))
    (else
      (Variables|CustomizationCamera|TouchDrag|SetLast_TouchDelta "")
      (bind _returnvalue (Utilities|Time|SetTimerbyEvent (EventDispatchers|CreateEvent :!event ResetRootOffset) (Variables|CustomizationCamera|GetCameraResetTime)))
      (Variables|CustomizationCamera|TouchDrag|SetRootOffsetReset_TimerHandle _returnvalue))))

(fn ResetRootOffset
  (Variables|CustomizationCamera|TouchDrag|SetTotal_TouchDelta "")
  (Utilities|Time|ClearandInvalidateTimerbyHandle (Variables|CustomizationCamera|TouchDrag|GetRootOffsetReset_TimerHandle)))

(fn ReceiveTick
  (params (DeltaSeconds :type Float%20%28single-precision%29))
  (Utilities|FlowControl|Sequence
    (:then_0
      (Variables|CustomizationCamera|TouchDrag|SetTotal_TouchDelta (Math|Vector2D|MakeVector2D (Class|KismetMathLibrary|ClampAxis (.X (Math|Vector2D|BreakVector2D (+ (Variables|CustomizationCamera|TouchDrag|GetTotal_TouchDelta) (Variables|CustomizationCamera|TouchDrag|GetLast_TouchDelta))))) (Class|KismetMathLibrary|ClampAxis (.Y (Math|Vector2D|BreakVector2D (+ (Variables|CustomizationCamera|TouchDrag|GetTotal_TouchDelta) (Variables|CustomizationCamera|TouchDrag|GetLast_TouchDelta))))))))
    (:then_1
      (Transformation|SetRelativeRotation (Variables|CustomizationCamera|Main|GetMeshRoot) (Math|Rotator|MakeRotator 0.0 0.0 (Math|Rotator|NormalizeAxis (.Yaw (Math|Rotator|BreakRotator (Math|Interpolation|RInterpTo (Variables|/Script/Engine.SceneComponent|GetRelativeRotation (Variables|CustomizationCamera|Main|GetMeshRoot)) (Math|Rotator|MakeRotator 0.0 0.0 (Class|KismetMathLibrary|ClampAxis (.x (Class|KismetMathLibrary|Negated2D (Variables|CustomizationCamera|TouchDrag|GetTotal_TouchDelta))))) (Utilities|Time|GetWorldDeltaSeconds) 5.0))))) false false))
    (:then_2
      (Utilities|FlowControl|Sequence
        (:then_0
          (if (Variables|CustomizationCamera|Data|GetUpdateCameraPosition)
            (goto _label Open)
            (else
              (CustomizationCamera|Update|CorrectCameraPosition)
              (goto _label Close))))
        (:then_1
          (Utilities|FlowControl|Gate true :!label _label
            (:Exit
              (bind _returnvalue (CustomizationCamera|Update|UpdateCameraCurve))
              (if _returnvalue
                (Variables|CustomizationCamera|Data|SetUpdateCameraPosition false)))))))))

(fn CorrectCameraPosition
  (bind _returnvalue (Components|GetOwner))
  (bind _camera (Variables|CustomizationCamera|Main|GetCamera))
  (bind _rootskeletalmeshcomponent (Variables|CustomizationCamera|Main|GetRootSkeletalMeshComponent))
  (bind _currentsettings (Variables|CustomizationCamera|Data|GetCurrentSettings))
  (bind _currentsettings_2 (Variables|CustomizationCamera|Data|GetCurrentSettings))
  (bind _rootskeletalmeshcomponent_2 (Variables|CustomizationCamera|Main|GetRootSkeletalMeshComponent))
  (bind _offset (Utilities|Struct|BreakStruct_CameraSettings _currentsettings))
  (bind _bonetotrack (Utilities|Struct|BreakStruct_CameraSettings _currentsettings_2))
  (bind _origin (Collision|GetComponentBounds _rootskeletalmeshcomponent_2))
  (bind _returnvalue_2 (Transformation|GetActorRightVector _returnvalue))
  (bind _returnvalue_3 (Transformation|GetActorForwardVector _returnvalue))
  (bind _returnvalue_4 (Math|Vector|NegateVector _returnvalue_3))
  (bind _returnvalue_5 (Transformation|GetSocketTransform _rootskeletalmeshcomponent _bonetotrack "RTS_Actor"))
  (bind _returnvalue_6 (* _returnvalue_2 (.y _offset)))
  (bind _returnvalue_7 (* _returnvalue_4 (.x _offset)))
  (bind _returnvalue_8 (+ (.location _returnvalue_5) _returnvalue_7 _returnvalue_6))
  (bind (_x _y) (Math|Vector|BreakVector _returnvalue_8))
  (Transformation|SetRelativeLocation _camera (Math|Interpolation|VInterpTo (Variables|/Script/Engine.SceneComponent|GetRelativeLocation _camera) (Math|Vector|MakeVector _x _y (+ (+ (.Z (Math|Vector|BreakVector _origin)) (Math|Float|Absolute(Float) (.Z (Math|Vector|BreakVector (- _origin (Transformation|GetSocketLocation (Variables|CustomizationCamera|Main|GetRootSkeletalMeshComponent) (Utilities|Struct|BreakStruct_CameraSettings (Variables|CustomizationCamera|Data|GetCurrentSettings)))))))) (.z _offset))) (Utilities|Time|GetWorldDeltaSeconds) 5.0) false false))

(fn TrySetViewTarget
  (if (Variables|CustomizationCamera|GetSetViewTargetOnBeginPlay)
    (Game|Player|SetViewTargetwithBlend (Game|GetPlayerController 0) (Components|GetOwner) 0.0 "VTBlend_Linear" 0.0 false)))