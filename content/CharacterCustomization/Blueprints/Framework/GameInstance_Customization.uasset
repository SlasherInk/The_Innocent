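; Game instance for the character customization system that owns the master menu widget and a reference to the customization pawn.
; TryCreateMenu lazily creates a single WB_MasterWidget for the local player controller, optionally adds it to the viewport, then loads main, in-game or pause menu content into it with transition animations.
; Each menu choice also sets the input mode and mouse cursor visibility on player controller 0.
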(fn AddMenutoViewport
  (params (Add :type Boolean))
  (if (and Add (not (UserInterface|Viewport|IsinViewport (Variables|Default|GetMasterWidget))))
    (UserInterface|Viewport|AddtoViewport (Variables|Default|GetMasterWidget) 0)
    (return true)))

(fn GetCustomizationPawn
  (return (Variables|Default|GetCustomizationPawn)))

(fn GetMasterMenu
  (return (Variables|Default|GetMasterWidget)))

(fn SetCustomizationPawn
  (params (Actor :type Actor%20Object%20Reference))
  (Variables|Default|SetCustomizationPawn Actor)
  (return (Utilities|IsValid (Variables|Default|GetCustomizationPawn))))

(fn TryCreateMenu
  (params (PlayerController :type Player%20Controller%20Object%20Reference) (TargetMenu :type Enum_MenuType%20Enum :default "NewEnumerator0") (AddToViewport :type Boolean))
  (if (Pawn|IsLocalPlayerController PlayerController)
    (Utilities|FlowControl|Sequence
      (:then_0
        (Variables|Default|GetMasterWidget
          (:then
            _)
          (:else
            (bind _returnvalue (UserInterface|CreateWidget "/Game/CharacterCustomization/UserInterface/Menu/WB_MasterWidget.WB_MasterWidget_C" PlayerController))
            (bind _output_get (Variables|Default|SetMasterWidget _returnvalue))
            (Default|OnConstructed _output_get)))
        (CallFunction|AddMenutoViewport AddToViewport))
      (:then_1
        (switch Utilities|FlowControl|Switch|SwitchonEnum_MenuType TargetMenu
          (:NewEnumerator0
            (Default|LoadContentfromClass (Variables|Default|GetMasterWidget) "/Game/CharacterCustomization/UserInterface/Menu/Content/WB_MainMenu.WB_MainMenu_C" "NewEnumerator0" "NewEnumerator2")
            (Input|SetInputModeUIOnly (Game|GetPlayerController 0) (Variables|Default|GetMasterWidget) "DoNotLock" false)
            (Variables|/Script/Engine.PlayerController|SetbShowMouseCursor (Game|GetPlayerController 0) true))
          (:NewEnumerator1
            (Default|LoadContentfromClass (Variables|Default|GetMasterWidget) "/Game/CharacterCustomization/UserInterface/Menu/Content/WB_Empty.WB_Empty_C" "NewEnumerator0" "NewEnumerator2")
            (Input|SetInputModeGameOnly (Game|GetPlayerController 0) false)
            (Variables|/Script/Engine.PlayerController|SetbShowMouseCursor (Game|GetPlayerController 0) false))
          (:NewEnumerator3
            (Default|LoadContentfromClass (Variables|Default|GetMasterWidget) "/Game/CharacterCustomization/UserInterface/Menu/Content/WB_PauseMenu.WB_PauseMenu_C" "NewEnumerator0" "NewEnumerator2")
            (Input|SetInputModeUIOnly (Game|GetPlayerController 0) (Variables|Default|GetMasterWidget) "DoNotLock" false)
            (Variables|/Script/Engine.PlayerController|SetbShowMouseCursor (Game|GetPlayerController 0) true))))
      (:then_2
        (return true)))))